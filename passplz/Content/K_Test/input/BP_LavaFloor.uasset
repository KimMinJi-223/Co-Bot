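; Destructible lava floor target in the Stage 3 cannon key hunt, melted by CPP_Lava projectiles.
; Each hit passes the projectile a render target bound to the floor's dynamic material to draw the melt.
; The third hit reveals whether a key is hidden, updating the signal color and triggering the clear sequence when complete.
; Otherwise hits spend controller shots, re-arming the cannon or, at zero, switching camera, setting capsules and enabling the portal.
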(event `self.ReceiveBeginPlay`
  (bind _returnvalue (`PrimitiveComponent.CreateDynamicMaterialInstance` (`self.StaticMesh`) 0 "/Game/K_Test/input/m_lava_Inst.m_lava_Inst" "None"))
  (set `self.m_lava` _returnvalue)
  (bind _returnvalue_2 (`KismetRenderingLibrary.CreateRenderTarget2D` 1024 1024))
  (set `self.dynamicRender` _returnvalue_2)
  (`MaterialInstanceDynamic.SetTextureParameterValue` (`self.m_lava`) "render" (`self.dynamicRender`)))

(event `self.ReceiveTick`
  (params (DeltaSeconds :type "Float (single-precision)"))
  (`/Engine/EditorBlueprintResources/StandardMacros.DoOnce` false
    (:`Completed`
      (bind _returnvalue (`GameplayStatics.GetActorOfClass` "/Game/K_Test/input/Cannon.Cannon_C"))
      (set `self.stage3Widget` (`/Game/K_Test/input/Cannon.stage3Widget` _returnvalue)))))

(event `self.StaticMesh.OnComponentBeginOverlap`
  (params (OverlappedComponent :type "PrimitiveComponent Object Reference") (OtherActor :type "Actor Object Reference") (OtherComp :type "PrimitiveComponent Object Reference") (OtherBodyIndex :type Integer) (bFromSweep :type Boolean) (SweepResult :type "HitResult Structure (by ref)"))
  (bind _keycolor (`self.keycolor`))
  (bind _stage3widget (`self.stage3Widget`))
  (bind _stage3widget_2 (`self.stage3Widget`))
  (bind _stage3widget_3 (`self.stage3Widget`))
  (bind _keynumber (`/Game/3S_BP/keyColor.keynumber` _keycolor))
  (bind _nokey (`/Game/widget/widget_Cannon.NoKey` _stage3widget_2))
  (bind _yeskey (`/Game/widget/widget_Cannon.YesKey` _stage3widget_2))
  (bind _success (`/Game/widget/widget_Cannon.success` _stage3widget_2))
  ;[1 1 1] 렌더타겟에 그림그리고 파티클
  (`|ExecutionSequence`
    (:`then_0`
      (bind _ascpp_lava (cast `CPP_Lava` OtherActor))
      (`GameplayStatics.PlaySound2D` "/Game/game_sound/missile_explosion.missile_explosion" 1.0 1.0 0.0 null null)
      (`PrimitiveComponent.SetCollisionEnabled` (`CPP_Lava.CollisionComponent` _ascpp_lava) "NoCollision")
      (set `CPP_Lava.RenderTargetTexture` (`self.dynamicRender`) _ascpp_lava)
      (`CPP_Lava.MeltLavaFloorLocation` _ascpp_lava)
      (`GameplayStatics.SpawnEmitterAtLocation` "/Game/StarterContent/Particles/P_Explosion.P_Explosion" (- SweepResult_Location (0.0 0.0 100.0)) (struct) (5.0 5.0 5.0))
      (`/Engine/EditorBlueprintResources/StandardMacros.IncrementInt` (`self.count`)
        (:`  `
          ;[1 1 1] true면 다른 곳을 쏘라는 위젯 이것이 true라면 횟수 차감이 없다.
          (if (> (`self.count`) 3)
            _
            (elif (== (`self.count`) 3)
              ;[1 1 1] 하나의 floor가 3발 모두 맞아고 키가 있는 곳인지 없는 곳인지 판단
              (if (`self.hasKey`)
                (set `TextBlock.Text` "열쇠를 찾았다!!!" _success)
                (`UserWidget.PlayAnimation` _stage3widget_2 _yeskey 0.0 1 "Forward" 1.0 false)
                (`KismetSystemLibrary.Delay` 1.0)
                (`PlayerController.SetViewTargetWithBlend` (`GameplayStatics.GetPlayerController` 0) (`self.camera1`) 1.0 "VTBlend_Linear" 0.0 false)
                (`KismetSystemLibrary.Delay` 1.5)
                ;[1 1 1] 신호등 색 바꾸기
                (`UserWidget.PlayAnimation` _stage3widget_2 _yeskey 0.0 1 "Reverse" 1.0 false)
                (`/Engine/EditorBlueprintResources/StandardMacros.IncrementInt` (`/Game/3S_BP/keyColor.keynumber` _keycolor)
                  (:`  `
                    (`MaterialInstanceDynamic.SetVectorParameterValue` (`/Game/3S_BP/keyColor.m_Color` _keycolor) "color" (`|GetArrayItem` (`/Game/3S_BP/keyColor.colors` _keycolor) _keynumber))
                    (if (== _keynumber 1)
                      (`UserWidget.PlayAnimation` _stage3widget (`/Game/widget/widget_Cannon.fire` _stage3widget) 0.0 1 "Reverse" 1.0 false)
                      ;[1 1 1] 미션 클리어
                      (`KismetSystemLibrary.Delay` 2.0)
                      (`PlayerController.SetViewTargetWithBlend` (`GameplayStatics.GetPlayerController` 0) (`self.camera2`) 1.0 "VTBlend_Linear" 0.0 false)
                      (bind _ascpp_cobot_car (cast `CPP_Cobot_Car` (`GameplayStatics.GetPlayerPawn` 0)))
                      (`/Game/3S_BP/keyColor.Floor_Move` (`self.keycolor`))
                      (`KismetSystemLibrary.Delay` 6.0)
                      (bind _returnvalue (`GameplayStatics.GetActorOfClass` "/Game/K_Test/input/Cannon.Cannon_C"))
                      (`/Game/K_Test/input/Cannon.Switch_Camera` _returnvalue)
                      (bind _returnvalue_2 (`GameplayStatics.GetActorOfClass` "/Game/Global_BP/Clear.Clear_C"))
                      (`/Game/Global_BP/Clear.Clear` _returnvalue_2)
                      (else
                        ;[1 1 1] 한 용암당 발사횟수는 3번이다 이를 줄이는 작업 fireNumㅇ이 0이된다면 모드를 바꾼다.
                        (bind _ascpp_cobot_car_controller (cast `CPP_Cobot_Car_Controller` (`GameplayStatics.GetPlayerController` 0) :!label _label))
                        (`/Engine/EditorBlueprintResources/StandardMacros.DecrementInt` (`CPP_Cobot_Car_Controller.fireNum` _ascpp_cobot_car_controller)
                          (:`  `
                            (bind _firenum (`CPP_Cobot_Car_Controller.fireNum` _ascpp_cobot_car_controller))
                            (bind _output (`|GetArrayItem` (`/Game/widget/widget_Cannon.fireimage` (`self.stage3Widget`)) _firenum))
                            (`UserWidget.PlayAnimation` _output (`/Game/widget/widget_fire.end` _output) 0.0 1 "Forward" 1.0 false)
                            (if (== _firenum 0)
                              (`UserWidget.PlayAnimation` _stage3widget_3 (`/Game/widget/widget_Cannon.fire` _stage3widget_3) 0.0 1 "Reverse" 1.0 false)
                              (bind _returnvalue_3 (`GameplayStatics.GetActorOfClass` "/Game/K_Test/input/Cannon.Cannon_C"))
                              (`/Game/K_Test/input/Cannon.Switch_Camera` _returnvalue_3)
                              (bind _outactors (`GameplayStatics.GetAllActorsOfClass` "/Game/3S_BP/Capsule.Capsule_C"))
                              (for _array_element _outactors
                                (`/Game/3S_BP/Capsule.SetCapsule` _array_element)
                                (bind _asnext_map (cast `/Game/3S_BP/next_map` (`self.potal`)))
                                (`PrimitiveComponent.SetCollisionEnabled` (`/Game/3S_BP/next_map.Box` _asnext_map) "QueryOnly")
                                (`SceneComponent.SetVisibility` (`/Game/3S_BP/next_map.Niagara` _asnext_map) true false))
                              (else
                                (`KismetSystemLibrary.Delay` 1.5)
                                (bind _returnvalue_4 (`GameplayStatics.GetActorOfClass` "/Game/K_Test/input/Cannon.Cannon_C"))
                                (`PlayerController.SetViewTargetWithBlend` (`GameplayStatics.GetPlayerController` 0) (`ActorComponent.GetOwner` (`/Game/K_Test/input/Cannon.Camera` _returnvalue_4)) 1.0 "VTBlend_Linear" 0.0 false)
                                (bind _ascpp_cobot_car_controller_2 (cast `CPP_Cobot_Car_Controller` (`GameplayStatics.GetPlayerController` 0)))
                                (`/Game/widget/widget_Cannon.uncheck` (`self.stage3Widget`))
                                (set `CPP_Cobot_Car_Controller.isFire` true _ascpp_cobot_car_controller_2)))))))))
                (else
                  (set `TextBlock.Text` "열쇠가 없네..." _success)
                  (`UserWidget.PlayAnimation` _stage3widget_2 _nokey 0.0 1 "Forward" 1.0 false)
                  (`KismetSystemLibrary.Delay` 2.5)
                  (`UserWidget.PlayAnimation` _stage3widget_2 _nokey 0.0 1 "Reverse" 1.0 false)
                  (goto _label)))
              (else
                (goto _label)))))))))

(fn `UserConstructionScript`)