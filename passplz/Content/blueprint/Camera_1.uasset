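; Camera actor that frames the COBOT actors, following them as they move.
; Every Tick it gathers all COBOTs into a location array and, inside that same loop, turns side-on to the line between the first two with a slight downward pitch.
; It then moves back along its forward vector from the average location by a fixed offset plus the pair's separation, so it pulls out as they spread apart.
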(event `self.ReceiveTick`
  (params (DeltaSeconds :type "Float (single-precision)"))
  (bind _returnvalue (`self.GetActorForwardVector`))
  (bind _cobot_location (`self.Cobot_location`))
  (bind _cobot_location_2 (`self.COBOT_location`))
  (bind (_returnvalue_x _returnvalue_y) (`KismetMathLibrary.BreakVector` (- (`|GetArrayItem` _cobot_location 1) (`|GetArrayItem` _cobot_location))))
  (bind (_returnvalue_roll _returnvalue_pitch _returnvalue_yaw) (`KismetMathLibrary.BreakRotator` (`KismetMathLibrary.MakeRotFromXY` (`KismetMathLibrary.MakeVector` _returnvalue_y (* _returnvalue_x -1.0)) (`KismetMathLibrary.MakeVector` _returnvalue_x _returnvalue_y))))
  (bind _outactors (`GameplayStatics.GetAllActorsOfClass` "/Game/blueprint/COBOT.COBOT_C"))
  (for (_array_element _array_index) _outactors
    (`KismetArrayLibrary.Array_Set` (`self.Cobot_location`) _array_index (`self.K2_GetActorLocation` _array_element))
    (`self.K2_SetActorRotation` (`KismetMathLibrary.MakeRotator` 0.0 -15.0 _returnvalue_yaw))
    (bind _output_get (set `self.for_camera_fov` (- (`|GetArrayItem` _cobot_location_2) (`|GetArrayItem` _cobot_location_2 1))))
    (`self.K2_SetActorLocation` (+ (* _returnvalue -400) (`KismetMathLibrary.GetVectorArrayAverage` _cobot_location) (* _returnvalue (* (`KismetMathLibrary.Sqrt` (+ (`KismetMathLibrary.Square` (.x _output_get)) (`KismetMathLibrary.Square` (.y _output_get)) (`KismetMathLibrary.Square` (.z _output_get)))) -1.0))))))

(fn `UserConstructionScript`)