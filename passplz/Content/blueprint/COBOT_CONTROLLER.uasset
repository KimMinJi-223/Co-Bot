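; COBOT_CONTROLLER is a player controller that drives its possessed pawn through two input axes.
; MOVE_FORWARD adds movement input to the pawn along the forward vector of the control rotation's yaw, ignoring pitch and roll.
; ROTATE adds yaw input scaled by frame delta time and a fixed turn multiplier, so turning also steers the direction of forward movement.
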(event `InputAxis|MOVE_FORWARD`
  (params (AxisValue :type "Float (single-precision)"))
  (bind _returnvalue (`self.K2_GetPawn`))
  (`/Engine/EditorBlueprintResources/StandardMacros.IsValid` _returnvalue
    (:`Is Valid`
      (`Pawn.AddMovementInput` _returnvalue (`KismetMathLibrary.GetForwardVector` (`KismetMathLibrary.MakeRotator` 0.0 0.0 (.yaw (`self.GetControlRotation`)))) AxisValue false))))

(event `InputAxis|ROTATE`
  (params (AxisValue :type "Float (single-precision)"))
  (`self.AddYawInput` (* AxisValue (`GameplayStatics.GetWorldDeltaSeconds`) 20.0)))

(fn `UserConstructionScript`)