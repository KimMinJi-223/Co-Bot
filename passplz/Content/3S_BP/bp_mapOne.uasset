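; Map blueprint for a one-stroke path puzzle where five paths link nodes A to D and each must be traversed once to open a door.
; Node overlaps, on begin and end, mark path endpoints and print "fail" when no connected path remains before clearing.
; Tick raises a path with both ends marked, clears all marks, and lifts the door once every path is used.
; A bound reset event restores paths and teleports the CPP_Cobot.
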(event `self.ReceiveBeginPlay`
  (bind _ad (`self.AD`))
  (bind _ab (`self.AB`))
  (bind _cd (`self.CD`))
  (bind _bd (`self.BD`))
  (bind _ac (`self.AC`))
  (`|ExecutionSequence`
    (:`then_0`
      (setmembers `/Game/3S_BP/struct_forMap` :`StructRef` (`self.infoAD`) :`path` _ad :`flag` 1 :`Pos1` false :`Pos2` false :`initialLocation` (`SceneComponent.K2_GetComponentLocation` _ad))
      (setmembers `/Game/3S_BP/struct_forMap` :`StructRef` (`self.infoCD`) :`path` _cd :`flag` 1 :`Pos1` false :`Pos2` false :`initialLocation` (`SceneComponent.K2_GetComponentLocation` _cd))
      (setmembers `/Game/3S_BP/struct_forMap` :`StructRef` (`self.infoBD`) :`path` _bd :`flag` 1 :`Pos1` false :`Pos2` false :`initialLocation` (`SceneComponent.K2_GetComponentLocation` _bd))
      (setmembers `/Game/3S_BP/struct_forMap` :`StructRef` (`self.infoAB`) :`path` _ab :`flag` 1 :`Pos1` false :`Pos2` false :`initialLocation` (`SceneComponent.K2_GetComponentLocation` _ab))
      (setmembers `/Game/3S_BP/struct_forMap` :`StructRef` (`self.infoAC`) :`path` _ac :`flag` 1 :`Pos1` false :`Pos2` false :`initialLocation` (`SceneComponent.K2_GetComponentLocation` _ac)))
    (:`then_1`
      (set `self.paths` (`|MakeArray` (`self.infoAD`) (`self.infoCD`) (`self.infoBD`) (`self.infoAB`) (`self.infoAC`))))
    (:`then_2`
      (add `self.reset` (delegate `reset_Event`)))))

(event `reset_Event`
  (`KismetSystemLibrary.PrintString` "reset")
  (bind _returnvalue (`GameplayStatics.GetActorOfClass` "/Script/passplz.CPP_Cobot"))
  (`self.K2_SetActorLocationAndRotation` :`self` _returnvalue :`NewLocation` (-2110.081029 12.654485 50.0) :`bTeleport` true)
  (for (_array_element _array_index) (`self.paths`)
    (bind (_path _flag _pos1 _pos2 _initiallocation) (break `/Game/3S_BP/struct_forMap` _array_element))
    (setmembers `/Game/3S_BP/struct_forMap` :`StructRef` (`|GetArrayItem` (`self.paths`) _array_index) :`path` _path :`flag` 1 :`Pos1` false :`Pos2` false :`initialLocation` _initiallocation)
    (`SceneComponent.K2_SetWorldLocation` _path _initiallocation false false)))

(event `self.ReceiveTick`
  (params (DeltaSeconds :type "Float (single-precision)"))
  (bind _checkifclear (`self.checkIfClear`))
  (bind _door (`self.door`))
  (`|ExecutionSequence`
    (:`then_0`
      (for (_array_element _array_index) (`self.paths`)
        (bind (_path _flag _pos1 _pos2 _initiallocation) (break `/Game/3S_BP/struct_forMap` _array_element))
        (if (and _pos1 _pos2)
          (`SceneComponent.K2_SetWorldLocation` _path (+ (`SceneComponent.K2_GetComponentLocation` _path) (0.0 0.0 500.0)) false false)
          (for (_array_element_2 _array_index_2) (`self.paths`)
            (bind (_path_2 _flag_2 _pos1_2 _pos2_2 _initiallocation_2) (break `/Game/3S_BP/struct_forMap` _array_element_2))
            (setmembers `/Game/3S_BP/struct_forMap` :`StructRef` (`|GetArrayItem` (`self.paths`) _array_index_2) :`path` _path_2 :`flag` _flag_2 :`Pos1` false :`Pos2` false :`initialLocation` _initiallocation_2))
          (setmembers `/Game/3S_BP/struct_forMap` :`StructRef` (`|GetArrayItem` (`self.paths`) _array_index) :`path` _path :`flag` 0 :`Pos1` false :`Pos2` false :`initialLocation` _initiallocation)
          (break))))
    (:`then_1`
      (for _array_element_3 (`self.paths`)
        (if (== 0 (`.flag_10_0196EC294EE995B605FDA4B4F36C79DF` (break `/Game/3S_BP/struct_forMap` _array_element_3)))
          (set `self.checkIfClear` (+ 1 _checkifclear))
          (if (== (`KismetArrayLibrary.Array_Length` (`self.paths`)) _checkifclear)
            (`SceneComponent.K2_SetWorldLocation` _door (+ (`SceneComponent.K2_GetComponentLocation` _door) (0.0 0.0 500.0)) false false)
            (set `self.clear ?` true)
            (`KismetSystemLibrary.PrintString` "clear"))))
      (set `self.checkIfClear` 0))))

(event `self.collision_A.OnComponentBeginOverlap`
  (params (OverlappedComponent :type "PrimitiveComponent Object Reference") (OtherActor :type "Actor Object Reference") (OtherComp :type "PrimitiveComponent Object Reference") (OtherBodyIndex :type Integer) (bFromSweep :type Boolean) (SweepResult :type "HitResult Structure (by ref)"))
  (bind _output (`|GetArrayItem` (`self.paths`) 4))
  (bind _output_2 (`|GetArrayItem` (`self.paths`)))
  (bind _output_3 (`|GetArrayItem` (`self.paths`) 3))
  (bind (_path _flag _pos1 _pos2 _initiallocation) (break `/Game/3S_BP/struct_forMap` _output_2))
  (bind (_path_2 _flag_2 _pos1_2 _pos2_2 _initiallocation_2) (break `/Game/3S_BP/struct_forMap` _output_3))
  (bind (_path_3 _flag_3 _pos1_3 _pos2_3 _initiallocation_3) (break `/Game/3S_BP/struct_forMap` _output))
  (setmembers `/Game/3S_BP/struct_forMap` :`StructRef` _output_2 :`path` _path :`flag` _flag :`Pos1` true :`Pos2` _pos2 :`initialLocation` _initiallocation :!label _label)
  (setmembers `/Game/3S_BP/struct_forMap` :`StructRef` _output_3 :`path` _path_2 :`flag` _flag_2 :`Pos1` true :`Pos2` _pos2_2 :`initialLocation` _initiallocation_2)
  (setmembers `/Game/3S_BP/struct_forMap` :`StructRef` _output :`path` _path_3 :`flag` _flag_3 :`Pos1` true :`Pos2` _pos2_3 :`initialLocation` _initiallocation_3)
  (if (and (!= (`self.clear ?`) true) (== (+ _flag_3 _flag_2 _flag) 0))
    (`KismetSystemLibrary.PrintString` "fail" true true (struct :`R` 1.0 :`A` 1.0))))

(event `self.collision_A.OnComponentEndOverlap`
  (params (OverlappedComponent :type "PrimitiveComponent Object Reference") (OtherActor :type "Actor Object Reference") (OtherComp :type "PrimitiveComponent Object Reference") (OtherBodyIndex :type Integer))
  (goto _label))

(event `self.collision_B.OnComponentBeginOverlap`
  (params (OverlappedComponent :type "PrimitiveComponent Object Reference") (OtherActor :type "Actor Object Reference") (OtherComp :type "PrimitiveComponent Object Reference") (OtherBodyIndex :type Integer) (bFromSweep :type Boolean) (SweepResult :type "HitResult Structure (by ref)"))
  (bind _output (`|GetArrayItem` (`self.paths`) 2))
  (bind _output_2 (`|GetArrayItem` (`self.paths`) 3))
  (bind (_path _flag _pos1 _pos2 _initiallocation) (break `/Game/3S_BP/struct_forMap` _output))
  (bind (_path_2 _flag_2 _pos1_2 _pos2_2 _initiallocation_2) (break `/Game/3S_BP/struct_forMap` _output_2))
  (setmembers `/Game/3S_BP/struct_forMap` :`StructRef` _output :`path` _path :`flag` _flag :`Pos1` true :`Pos2` _pos2 :`initialLocation` _initiallocation :!label _label_2)
  (setmembers `/Game/3S_BP/struct_forMap` :`StructRef` _output_2 :`path` _path_2 :`flag` _flag_2 :`Pos1` _pos1_2 :`Pos2` true :`initialLocation` _initiallocation_2)
  (if (and (!= (`self.clear ?`) true) (== (+ _flag_2 _flag) 0))
    (`KismetSystemLibrary.PrintString` "fail" true true (struct :`R` 1.0 :`A` 1.0))))

(event `self.collision_B.OnComponentEndOverlap`
  (params (OverlappedComponent :type "PrimitiveComponent Object Reference") (OtherActor :type "Actor Object Reference") (OtherComp :type "PrimitiveComponent Object Reference") (OtherBodyIndex :type Integer))
  (goto _label_2))

(event `self.collision_C.OnComponentBeginOverlap`
  (params (OverlappedComponent :type "PrimitiveComponent Object Reference") (OtherActor :type "Actor Object Reference") (OtherComp :type "PrimitiveComponent Object Reference") (OtherBodyIndex :type Integer) (bFromSweep :type Boolean) (SweepResult :type "HitResult Structure (by ref)"))
  (bind _output (`|GetArrayItem` (`self.paths`) 1))
  (bind _output_2 (`|GetArrayItem` (`self.paths`) 4))
  (bind (_path _flag _pos1 _pos2 _initiallocation) (break `/Game/3S_BP/struct_forMap` _output))
  (bind (_path_2 _flag_2 _pos1_2 _pos2_2 _initiallocation_2) (break `/Game/3S_BP/struct_forMap` _output_2))
  (setmembers `/Game/3S_BP/struct_forMap` :`StructRef` _output :`path` _path :`flag` _flag :`Pos1` true :`Pos2` _pos2 :`initialLocation` _initiallocation :!label _label_3)
  (setmembers `/Game/3S_BP/struct_forMap` :`StructRef` _output_2 :`path` _path_2 :`flag` _flag_2 :`Pos1` _pos1_2 :`Pos2` true :`initialLocation` _initiallocation_2)
  (if (and (!= (`self.clear ?`) true) (== (+ _flag_2 _flag) 0))
    (`KismetSystemLibrary.PrintString` "fail" true true (struct :`R` 1.0 :`A` 1.0))))

(event `self.collision_C.OnComponentEndOverlap`
  (params (OverlappedComponent :type "PrimitiveComponent Object Reference") (OtherActor :type "Actor Object Reference") (OtherComp :type "PrimitiveComponent Object Reference") (OtherBodyIndex :type Integer))
  (goto _label_3))

(event `self.collision_D.OnComponentBeginOverlap`
  (params (OverlappedComponent :type "PrimitiveComponent Object Reference") (OtherActor :type "Actor Object Reference") (OtherComp :type "PrimitiveComponent Object Reference") (OtherBodyIndex :type Integer) (bFromSweep :type Boolean) (SweepResult :type "HitResult Structure (by ref)"))
  (bind _output (`|GetArrayItem` (`self.paths`) 2))
  (bind _output_2 (`|GetArrayItem` (`self.paths`)))
  (bind _output_3 (`|GetArrayItem` (`self.paths`) 1))
  (bind (_path _flag _pos1 _pos2 _initiallocation) (break `/Game/3S_BP/struct_forMap` _output))
  (bind (_path_2 _flag_2 _pos1_2 _pos2_2 _initiallocation_2) (break `/Game/3S_BP/struct_forMap` _output_2))
  (bind (_path_3 _flag_3 _pos1_3 _pos2_3 _initiallocation_3) (break `/Game/3S_BP/struct_forMap` _output_3))
  (setmembers `/Game/3S_BP/struct_forMap` :`StructRef` _output_2 :`path` _path_2 :`flag` _flag_2 :`Pos1` _pos1_2 :`Pos2` true :`initialLocation` _initiallocation_2 :!label _label_4)
  (setmembers `/Game/3S_BP/struct_forMap` :`StructRef` _output_3 :`path` _path_3 :`flag` _flag_3 :`Pos1` _pos1_3 :`Pos2` true :`initialLocation` _initiallocation_3)
  (setmembers `/Game/3S_BP/struct_forMap` :`StructRef` _output :`path` _path :`flag` _flag :`Pos1` _pos1 :`Pos2` true :`initialLocation` _initiallocation)
  (if (and (!= (`self.clear ?`) true) (== (+ _flag _flag_3 _flag_2) 0))
    (`KismetSystemLibrary.PrintString` "fail" true true (struct :`R` 1.0 :`A` 1.0))))

(event `self.collision_D.OnComponentEndOverlap`
  (params (OverlappedComponent :type "PrimitiveComponent Object Reference") (OtherActor :type "Actor Object Reference") (OtherComp :type "PrimitiveComponent Object Reference") (OtherBodyIndex :type Integer))
  (goto _label_4))

(fn `UserConstructionScript`)