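; Map five puzzle Blueprint where every path linking lettered nodes A to L must be used once to open the door.
; Node collision overlaps mark ends of adjacent paths; Tick lifts any path with both ends marked, zeroes its flag and clears all marks.
; All flags at zero raise the door, while a node with spent paths prints "fail" before completion.
; A bound reset event restores the paths and teleports CPP_Cobot back.
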(event `self.ReceiveBeginPlay`
  (bind _ek (`self.EK`))
  (bind _cf (`self.CF`))
  (bind _dk (`self.DK`))
  (bind _cl (`self.CL`))
  (bind _fj (`self.FJ`))
  (bind _bj (`self.BJ`))
  (bind _bi (`self.BI`))
  (bind _gk (`self.GK`))
  (bind _gi (`self.GI`))
  (bind _dl (`self.DL`))
  (bind _ck (`self.CK`))
  (bind _be (`self.BE`))
  (bind _aj (`self.AJ`))
  (bind _ai (`self.AI`))
  (bind _hj (`self.HJ`))
  (bind _hl (`self.HL`))
  (`|ExecutionSequence`
    (:`then_0`
      (setmembers `/Game/3S_BP/struct_forMap` :`StructRef` (`self.infoCK`) :`path` _ck :`flag` 1 :`Pos1` false :`Pos2` false :`initialLocation` (`SceneComponent.K2_GetComponentLocation` _ck))
      (setmembers `/Game/3S_BP/struct_forMap` :`StructRef` (`self.infoHL`) :`path` _hl :`flag` 1 :`Pos1` false :`Pos2` false :`initialLocation` (`SceneComponent.K2_GetComponentLocation` _hl))
      (setmembers `/Game/3S_BP/struct_forMap` :`StructRef` (`self.infoEK`) :`path` _ek :`flag` 1 :`Pos1` false :`Pos2` false :`initialLocation` (`SceneComponent.K2_GetComponentLocation` _ek))
      (setmembers `/Game/3S_BP/struct_forMap` :`StructRef` (`self.infoCF`) :`path` _cf :`flag` 1 :`Pos1` false :`Pos2` false :`initialLocation` (`SceneComponent.K2_GetComponentLocation` _cf))
      (setmembers `/Game/3S_BP/struct_forMap` :`StructRef` (`self.infoDK`) :`path` _dk :`flag` 1 :`Pos1` false :`Pos2` false :`initialLocation` (`SceneComponent.K2_GetComponentLocation` _dk))
      (setmembers `/Game/3S_BP/struct_forMap` :`StructRef` (`self.infoCL`) :`path` _cl :`flag` 1 :`Pos1` false :`Pos2` false :`initialLocation` (`SceneComponent.K2_GetComponentLocation` _cl))
      (setmembers `/Game/3S_BP/struct_forMap` :`StructRef` (`self.infoFJ`) :`path` _fj :`flag` 1 :`Pos1` false :`Pos2` false :`initialLocation` (`SceneComponent.K2_GetComponentLocation` _fj))
      (setmembers `/Game/3S_BP/struct_forMap` :`StructRef` (`self.infoBJ`) :`path` _bj :`flag` 1 :`Pos1` false :`Pos2` false :`initialLocation` (`SceneComponent.K2_GetComponentLocation` _bj))
      (setmembers `/Game/3S_BP/struct_forMap` :`StructRef` (`self.infoBI`) :`path` _bi :`flag` 1 :`Pos1` false :`Pos2` false :`initialLocation` (`SceneComponent.K2_GetComponentLocation` _bi))
      (setmembers `/Game/3S_BP/struct_forMap` :`StructRef` (`self.infoGK`) :`path` _gk :`flag` 1 :`Pos1` false :`Pos2` false :`initialLocation` (`SceneComponent.K2_GetComponentLocation` _gk))
      (setmembers `/Game/3S_BP/struct_forMap` :`StructRef` (`self.infoGI`) :`path` _gi :`flag` 1 :`Pos1` false :`Pos2` false :`initialLocation` (`SceneComponent.K2_GetComponentLocation` _gi))
      (setmembers `/Game/3S_BP/struct_forMap` :`StructRef` (`self.infoDL`) :`path` _dl :`flag` 1 :`Pos1` false :`Pos2` false :`initialLocation` (`SceneComponent.K2_GetComponentLocation` _dl))
      (setmembers `/Game/3S_BP/struct_forMap` :`StructRef` (`self.infoBE`) :`path` _be :`flag` 1 :`Pos1` false :`Pos2` false :`initialLocation` (`SceneComponent.K2_GetComponentLocation` _be))
      (setmembers `/Game/3S_BP/struct_forMap` :`StructRef` (`self.infoAJ`) :`path` _aj :`flag` 1 :`Pos1` false :`Pos2` false :`initialLocation` (`SceneComponent.K2_GetComponentLocation` _aj))
      (setmembers `/Game/3S_BP/struct_forMap` :`StructRef` (`self.infoAI`) :`path` _ai :`flag` 1 :`Pos1` false :`Pos2` false :`initialLocation` (`SceneComponent.K2_GetComponentLocation` _ai))
      (setmembers `/Game/3S_BP/struct_forMap` :`StructRef` (`self.infoHJ`) :`path` _hj :`flag` 1 :`Pos1` false :`Pos2` false :`initialLocation` (`SceneComponent.K2_GetComponentLocation` _hj)))
    (:`then_1`
      (set `self.paths` (`|MakeArray` (`self.infoCK`) (`self.infoHL`) (`self.infoEK`) (`self.infoCF`) (`self.infoDK`) (`self.infoCL`) (`self.infoFJ`) (`self.infoBJ`) (`self.infoBI`) (`self.infoGK`) (`self.infoGI`) (`self.infoDL`) (`self.infoBE`) (`self.infoAJ`) (`self.infoAI`) (`self.infoHJ`))))
    (:`then_2`
      (add `self.reset` (delegate `reset_Event`)))))

(event `reset_Event`
  (`KismetSystemLibrary.PrintString` "reset")
  (bind _returnvalue (`GameplayStatics.GetActorOfClass` "/Script/passplz.CPP_Cobot"))
  (`self.K2_SetActorLocationAndRotation` :`self` _returnvalue :`NewLocation` (-2110.081029 12.654485 50.0) :`bTeleport` true)
  (for (_array_element _array_index) (`self.paths`)
    (bind (_path _flag _pos1 _pos2 _initiallocation) (break `/Game/3S_BP/struct_forMap` _array_element))
    (setmembers `/Game/3S_BP/struct_forMap` :`StructRef` (`|GetArrayItem` (`self.paths`) _array_index) :`path` _path :`flag` 1 :`Pos1` false :`Pos2` false :`initialLocation` _initiallocation)
    (`SceneComponent.K2_SetWorldLocation` _path _initiallocation false false)))

(event `self.ReceiveTick`
  (params (DeltaSeconds :type "Float (single-precision)"))
  (bind _checkifclear (`self.checkIfClear`))
  (bind _door (`self.door`))
  (`|ExecutionSequence`
    (:`then_0`
      (for (_array_element _array_index) (`self.paths`)
        (bind (_path _flag _pos1 _pos2 _initiallocation) (break `/Game/3S_BP/struct_forMap` _array_element))
        (if (and _pos1 _pos2)
          (`SceneComponent.K2_SetWorldLocation` _path (+ (`SceneComponent.K2_GetComponentLocation` _path) (0.0 0.0 500.0)) false false)
          (for (_array_element_2 _array_index_2) (`self.paths`)
            (bind (_path_2 _flag_2 _pos1_2 _pos2_2 _initiallocation_2) (break `/Game/3S_BP/struct_forMap` _array_element_2))
            (setmembers `/Game/3S_BP/struct_forMap` :`StructRef` (`|GetArrayItem` (`self.paths`) _array_index_2) :`path` _path_2 :`flag` _flag_2 :`Pos1` false :`Pos2` false :`initialLocation` _initiallocation_2))
          (setmembers `/Game/3S_BP/struct_forMap` :`StructRef` (`|GetArrayItem` (`self.paths`) _array_index) :`path` _path :`flag` 0 :`Pos1` false :`Pos2` false :`initialLocation` _initiallocation)
          (break))))
    (:`then_1`
      (for _array_element_3 (`self.paths`)
        (if (== 0 (`.flag_10_0196EC294EE995B605FDA4B4F36C79DF` (break `/Game/3S_BP/struct_forMap` _array_element_3)))
          (set `self.checkIfClear` (+ 1 _checkifclear))
          (if (== (`KismetArrayLibrary.Array_Length` (`self.paths`)) _checkifclear)
            (`SceneComponent.K2_SetWorldLocation` _door (+ (`SceneComponent.K2_GetComponentLocation` _door) (0.0 0.0 500.0)) false false)
            (set `self.clear ?` true)
            (`KismetSystemLibrary.PrintString` "clear"))))
      (set `self.checkIfClear` 0))))

(event `self.collision_A.OnComponentBeginOverlap`
  (params (OverlappedComponent :type "PrimitiveComponent Object Reference") (OtherActor :type "Actor Object Reference") (OtherComp :type "PrimitiveComponent Object Reference") (OtherBodyIndex :type Integer) (bFromSweep :type Boolean) (SweepResult :type "HitResult Structure (by ref)"))
  (bind _output (`|GetArrayItem` (`self.paths`) 14))
  (bind _output_2 (`|GetArrayItem` (`self.paths`) 13))
  (bind (_path _flag _pos1 _pos2 _initiallocation) (break `/Game/3S_BP/struct_forMap` _output))
  (bind (_path_2 _flag_2 _pos1_2 _pos2_2 _initiallocation_2) (break `/Game/3S_BP/struct_forMap` _output_2))
  (setmembers `/Game/3S_BP/struct_forMap` :`StructRef` _output :`path` _path :`flag` _flag :`Pos1` true :`Pos2` _pos2 :`initialLocation` _initiallocation :!label _label)
  (setmembers `/Game/3S_BP/struct_forMap` :`StructRef` _output_2 :`path` _path_2 :`flag` _flag_2 :`Pos1` true :`Pos2` _pos2_2 :`initialLocation` _initiallocation_2)
  (if (and (!= (`self.clear ?`) true) (== (+ _flag_2 _flag) 0))
    (`KismetSystemLibrary.PrintString` "fail" true true (struct :`R` 1.0 :`A` 1.0))))

(event `self.collision_A.OnComponentEndOverlap`
  (params (OverlappedComponent :type "PrimitiveComponent Object Reference") (OtherActor :type "Actor Object Reference") (OtherComp :type "PrimitiveComponent Object Reference") (OtherBodyIndex :type Integer))
  (goto _label))

(event `self.collision_B.OnComponentBeginOverlap`
  (params (OverlappedComponent :type "PrimitiveComponent Object Reference") (OtherActor :type "Actor Object Reference") (OtherComp :type "PrimitiveComponent Object Reference") (OtherBodyIndex :type Integer) (bFromSweep :type Boolean) (SweepResult :type "HitResult Structure (by ref)"))
  (bind _output (`|GetArrayItem` (`self.paths`) 7))
  (bind _output_2 (`|GetArrayItem` (`self.paths`) 8))
  (bind _output_3 (`|GetArrayItem` (`self.paths`) 12))
  (bind (_path _flag _pos1 _pos2 _initiallocation) (break `/Game/3S_BP/struct_forMap` _output))
  (bind (_path_2 _flag_2 _pos1_2 _pos2_2 _initiallocation_2) (break `/Game/3S_BP/struct_forMap` _output_2))
  (bind (_path_3 _flag_3 _pos1_3 _pos2_3 _initiallocation_3) (break `/Game/3S_BP/struct_forMap` _output_3))
  (setmembers `/Game/3S_BP/struct_forMap` :`StructRef` _output_2 :`path` _path_2 :`flag` _flag_2 :`Pos1` true :`Pos2` _pos2_2 :`initialLocation` _initiallocation_2 :!label _label_2)
  (setmembers `/Game/3S_BP/struct_forMap` :`StructRef` _output :`path` _path :`flag` _flag :`Pos1` true :`Pos2` _pos2 :`initialLocation` _initiallocation)
  (setmembers `/Game/3S_BP/struct_forMap` :`StructRef` _output_3 :`path` _path_3 :`flag` _flag_3 :`Pos1` true :`Pos2` _pos2_3 :`initialLocation` _initiallocation_3)
  (if (and (!= (`self.clear ?`) true) (== (+ _flag _flag_2 _flag_3) 0))
    (`KismetSystemLibrary.PrintString` "fail" true true (struct :`R` 1.0 :`A` 1.0))))

(event `self.collision_B.OnComponentEndOverlap`
  (params (OverlappedComponent :type "PrimitiveComponent Object Reference") (OtherActor :type "Actor Object Reference") (OtherComp :type "PrimitiveComponent Object Reference") (OtherBodyIndex :type Integer))
  (goto _label_2))

(event `self.collision_C.OnComponentBeginOverlap`
  (params (OverlappedComponent :type "PrimitiveComponent Object Reference") (OtherActor :type "Actor Object Reference") (OtherComp :type "PrimitiveComponent Object Reference") (OtherBodyIndex :type Integer) (bFromSweep :type Boolean) (SweepResult :type "HitResult Structure (by ref)"))
  (bind _output (`|GetArrayItem` (`self.paths`) 3))
  (bind _output_2 (`|GetArrayItem` (`self.paths`) 5))
  (bind _output_3 (`|GetArrayItem` (`self.paths`)))
  (bind (_path _flag _pos1 _pos2 _initiallocation) (break `/Game/3S_BP/struct_forMap` _output))
  (bind (_path_2 _flag_2 _pos1_2 _pos2_2 _initiallocation_2) (break `/Game/3S_BP/struct_forMap` _output_2))
  (bind (_path_3 _flag_3 _pos1_3 _pos2_3 _initiallocation_3) (break `/Game/3S_BP/struct_forMap` _output_3))
  (setmembers `/Game/3S_BP/struct_forMap` :`StructRef` _output :`path` _path :`flag` _flag :`Pos1` true :`Pos2` _pos2 :`initialLocation` _initiallocation :!label _label_3)
  (setmembers `/Game/3S_BP/struct_forMap` :`StructRef` _output_2 :`path` _path_2 :`flag` _flag_2 :`Pos1` true :`Pos2` _pos2_2 :`initialLocation` _initiallocation_2)
  (setmembers `/Game/3S_BP/struct_forMap` :`StructRef` _output_3 :`path` _path_3 :`flag` _flag_3 :`Pos1` true :`Pos2` _pos2_3 :`initialLocation` _initiallocation_3)
  (if (and (!= (`self.clear ?`) true) (== (+ _flag_2 _flag _flag_3) 0))
    (`KismetSystemLibrary.PrintString` "fail" true true (struct :`R` 1.0 :`A` 1.0))))

(event `self.collision_C.OnComponentEndOverlap`
  (params (OverlappedComponent :type "PrimitiveComponent Object Reference") (OtherActor :type "Actor Object Reference") (OtherComp :type "PrimitiveComponent Object Reference") (OtherBodyIndex :type Integer))
  (goto _label_3))

(event `self.collision_D.OnComponentBeginOverlap`
  (params (OverlappedComponent :type "PrimitiveComponent Object Reference") (OtherActor :type "Actor Object Reference") (OtherComp :type "PrimitiveComponent Object Reference") (OtherBodyIndex :type Integer) (bFromSweep :type Boolean) (SweepResult :type "HitResult Structure (by ref)"))
  (bind _output (`|GetArrayItem` (`self.paths`) 4))
  (bind _output_2 (`|GetArrayItem` (`self.paths`) 11))
  (bind (_path _flag _pos1 _pos2 _initiallocation) (break `/Game/3S_BP/struct_forMap` _output))
  (bind (_path_2 _flag_2 _pos1_2 _pos2_2 _initiallocation_2) (break `/Game/3S_BP/struct_forMap` _output_2))
  (setmembers `/Game/3S_BP/struct_forMap` :`StructRef` _output :`path` _path :`flag` _flag :`Pos1` true :`Pos2` _pos2 :`initialLocation` _initiallocation :!label _label_4)
  (setmembers `/Game/3S_BP/struct_forMap` :`StructRef` _output_2 :`path` _path_2 :`flag` _flag_2 :`Pos1` true :`Pos2` _pos2_2 :`initialLocation` _initiallocation_2)
  (if (and (!= (`self.clear ?`) true) (== (+ _flag_2 _flag) 0))
    (`KismetSystemLibrary.PrintString` "fail" true true (struct :`R` 1.0 :`A` 1.0))))

(event `self.collision_D.OnComponentEndOverlap`
  (params (OverlappedComponent :type "PrimitiveComponent Object Reference") (OtherActor :type "Actor Object Reference") (OtherComp :type "PrimitiveComponent Object Reference") (OtherBodyIndex :type Integer))
  (goto _label_4))

(event `self.collision_E.OnComponentBeginOverlap`
  (params (OverlappedComponent :type "PrimitiveComponent Object Reference") (OtherActor :type "Actor Object Reference") (OtherComp :type "PrimitiveComponent Object Reference") (OtherBodyIndex :type Integer) (bFromSweep :type Boolean) (SweepResult :type "HitResult Structure (by ref)"))
  (bind _output (`|GetArrayItem` (`self.paths`) 2))
  (bind _output_2 (`|GetArrayItem` (`self.paths`) 12))
  (bind (_path _flag _pos1 _pos2 _initiallocation) (break `/Game/3S_BP/struct_forMap` _output))
  (bind (_path_2 _flag_2 _pos1_2 _pos2_2 _initiallocation_2) (break `/Game/3S_BP/struct_forMap` _output_2))
  (setmembers `/Game/3S_BP/struct_forMap` :`StructRef` _output :`path` _path :`flag` _flag :`Pos1` true :`Pos2` _pos2 :`initialLocation` _initiallocation :!label _label_5)
  (setmembers `/Game/3S_BP/struct_forMap` :`StructRef` _output_2 :`path` _path_2 :`flag` _flag_2 :`Pos1` _pos1_2 :`Pos2` true :`initialLocation` _initiallocation_2)
  (if (and (!= (`self.clear ?`) true) (== (+ _flag_2 _flag) 0))
    (`KismetSystemLibrary.PrintString` "fail" true true (struct :`R` 1.0 :`A` 1.0))))

(event `self.collision_E.OnComponentEndOverlap`
  (params (OverlappedComponent :type "PrimitiveComponent Object Reference") (OtherActor :type "Actor Object Reference") (OtherComp :type "PrimitiveComponent Object Reference") (OtherBodyIndex :type Integer))
  (goto _label_5))

(event `self.collision_F.OnComponentBeginOverlap`
  (params (OverlappedComponent :type "PrimitiveComponent Object Reference") (OtherActor :type "Actor Object Reference") (OtherComp :type "PrimitiveComponent Object Reference") (OtherBodyIndex :type Integer) (bFromSweep :type Boolean) (SweepResult :type "HitResult Structure (by ref)"))
  (bind _output (`|GetArrayItem` (`self.paths`) 3))
  (bind _output_2 (`|GetArrayItem` (`self.paths`) 6))
  (bind (_path _flag _pos1 _pos2 _initiallocation) (break `/Game/3S_BP/struct_forMap` _output))
  (bind (_path_2 _flag_2 _pos1_2 _pos2_2 _initiallocation_2) (break `/Game/3S_BP/struct_forMap` _output_2))
  (setmembers `/Game/3S_BP/struct_forMap` :`StructRef` _output :`path` _path :`flag` _flag :`Pos1` _pos1 :`Pos2` true :`initialLocation` _initiallocation :!label _label_6)
  (setmembers `/Game/3S_BP/struct_forMap` :`StructRef` _output_2 :`path` _path_2 :`flag` _flag_2 :`Pos1` true :`Pos2` _pos2_2 :`initialLocation` _initiallocation_2)
  (if (and (!= (`self.clear ?`) true) (== (+ _flag_2 _flag) 0))
    (`KismetSystemLibrary.PrintString` "fail" true true (struct :`R` 1.0 :`A` 1.0))))

(event `self.collision_F.OnComponentEndOverlap`
  (params (OverlappedComponent :type "PrimitiveComponent Object Reference") (OtherActor :type "Actor Object Reference") (OtherComp :type "PrimitiveComponent Object Reference") (OtherBodyIndex :type Integer))
  (goto _label_6))

(event `self.collision_G.OnComponentBeginOverlap`
  (params (OverlappedComponent :type "PrimitiveComponent Object Reference") (OtherActor :type "Actor Object Reference") (OtherComp :type "PrimitiveComponent Object Reference") (OtherBodyIndex :type Integer) (bFromSweep :type Boolean) (SweepResult :type "HitResult Structure (by ref)"))
  (bind _output (`|GetArrayItem` (`self.paths`) 9))
  (bind _output_2 (`|GetArrayItem` (`self.paths`) 10))
  (bind (_path _flag _pos1 _pos2 _initiallocation) (break `/Game/3S_BP/struct_forMap` _output))
  (bind (_path_2 _flag_2 _pos1_2 _pos2_2 _initiallocation_2) (break `/Game/3S_BP/struct_forMap` _output_2))
  (setmembers `/Game/3S_BP/struct_forMap` :`StructRef` _output :`path` _path :`flag` _flag :`Pos1` true :`Pos2` _pos2 :`initialLocation` _initiallocation :!label _label_7)
  (setmembers `/Game/3S_BP/struct_forMap` :`StructRef` _output_2 :`path` _path_2 :`flag` _flag_2 :`Pos1` true :`Pos2` _pos2_2 :`initialLocation` _initiallocation_2)
  (if (and (!= (`self.clear ?`) true) (== (+ _flag_2 _flag) 0))
    (`KismetSystemLibrary.PrintString` "fail" true true (struct :`R` 1.0 :`A` 1.0))))

(event `self.collision_G.OnComponentEndOverlap`
  (params (OverlappedComponent :type "PrimitiveComponent Object Reference") (OtherActor :type "Actor Object Reference") (OtherComp :type "PrimitiveComponent Object Reference") (OtherBodyIndex :type Integer))
  (goto _label_7))

(event `self.collision_H.OnComponentBeginOverlap`
  (params (OverlappedComponent :type "PrimitiveComponent Object Reference") (OtherActor :type "Actor Object Reference") (OtherComp :type "PrimitiveComponent Object Reference") (OtherBodyIndex :type Integer) (bFromSweep :type Boolean) (SweepResult :type "HitResult Structure (by ref)"))
  (bind _output (`|GetArrayItem` (`self.paths`) 1))
  (bind _output_2 (`|GetArrayItem` (`self.paths`) 15))
  (bind (_path _flag _pos1 _pos2 _initiallocation) (break `/Game/3S_BP/struct_forMap` _output))
  (bind (_path_2 _flag_2 _pos1_2 _pos2_2 _initiallocation_2) (break `/Game/3S_BP/struct_forMap` _output_2))
  (setmembers `/Game/3S_BP/struct_forMap` :`StructRef` _output :`path` _path :`flag` _flag :`Pos1` true :`Pos2` _pos2 :`initialLocation` _initiallocation :!label _label_8)
  (setmembers `/Game/3S_BP/struct_forMap` :`StructRef` _output_2 :`path` _path_2 :`flag` _flag_2 :`Pos1` true :`Pos2` _pos2_2 :`initialLocation` _initiallocation_2)
  (if (and (!= (`self.clear ?`) true) (== (+ _flag_2 _flag) 0))
    (`KismetSystemLibrary.PrintString` "fail" true true (struct :`R` 1.0 :`A` 1.0))))

(event `self.collision_H.OnComponentEndOverlap`
  (params (OverlappedComponent :type "PrimitiveComponent Object Reference") (OtherActor :type "Actor Object Reference") (OtherComp :type "PrimitiveComponent Object Reference") (OtherBodyIndex :type Integer))
  (goto _label_8))

(event `self.collision_I.OnComponentBeginOverlap`
  (params (OverlappedComponent :type "PrimitiveComponent Object Reference") (OtherActor :type "Actor Object Reference") (OtherComp :type "PrimitiveComponent Object Reference") (OtherBodyIndex :type Integer) (bFromSweep :type Boolean) (SweepResult :type "HitResult Structure (by ref)"))
  (bind _output (`|GetArrayItem` (`self.paths`) 8))
  (bind _output_2 (`|GetArrayItem` (`self.paths`) 10))
  (bind _output_3 (`|GetArrayItem` (`self.paths`) 14))
  (bind (_path _flag _pos1 _pos2 _initiallocation) (break `/Game/3S_BP/struct_forMap` _output))
  (bind (_path_2 _flag_2 _pos1_2 _pos2_2 _initiallocation_2) (break `/Game/3S_BP/struct_forMap` _output_2))
  (bind (_path_3 _flag_3 _pos1_3 _pos2_3 _initiallocation_3) (break `/Game/3S_BP/struct_forMap` _output_3))
  (setmembers `/Game/3S_BP/struct_forMap` :`StructRef` _output :`path` _path :`flag` _flag :`Pos1` _pos1 :`Pos2` true :`initialLocation` _initiallocation :!label _label_9)
  (setmembers `/Game/3S_BP/struct_forMap` :`StructRef` _output_2 :`path` _path_2 :`flag` _flag_2 :`Pos1` _pos1_2 :`Pos2` true :`initialLocation` _initiallocation_2)
  (setmembers `/Game/3S_BP/struct_forMap` :`StructRef` _output_3 :`path` _path_3 :`flag` _flag_3 :`Pos1` _pos1_3 :`Pos2` true :`initialLocation` _initiallocation_3)
  (if (and (!= (`self.clear ?`) true) (== (+ _flag _flag_2 _flag_3) 0))
    (`KismetSystemLibrary.PrintString` "fail" true true (struct :`R` 1.0 :`A` 1.0))))

(event `self.collision_I.OnComponentEndOverlap`
  (params (OverlappedComponent :type "PrimitiveComponent Object Reference") (OtherActor :type "Actor Object Reference") (OtherComp :type "PrimitiveComponent Object Reference") (OtherBodyIndex :type Integer))
  (goto _label_9))

(event `self.collision_J.OnComponentBeginOverlap`
  (params (OverlappedComponent :type "PrimitiveComponent Object Reference") (OtherActor :type "Actor Object Reference") (OtherComp :type "PrimitiveComponent Object Reference") (OtherBodyIndex :type Integer) (bFromSweep :type Boolean) (SweepResult :type "HitResult Structure (by ref)"))
  (bind _output (`|GetArrayItem` (`self.paths`) 6))
  (bind _output_2 (`|GetArrayItem` (`self.paths`) 7))
  (bind _output_3 (`|GetArrayItem` (`self.paths`) 13))
  (bind _output_4 (`|GetArrayItem` (`self.paths`) 15))
  (bind (_path _flag _pos1 _pos2 _initiallocation) (break `/Game/3S_BP/struct_forMap` _output))
  (bind (_path_2 _flag_2 _pos1_2 _pos2_2 _initiallocation_2) (break `/Game/3S_BP/struct_forMap` _output_2))
  (bind (_path_3 _flag_3 _pos1_3 _pos2_3 _initiallocation_3) (break `/Game/3S_BP/struct_forMap` _output_3))
  (bind (_path_4 _flag_4 _pos1_4 _pos2_4 _initiallocation_4) (break `/Game/3S_BP/struct_forMap` _output_4))
  (setmembers `/Game/3S_BP/struct_forMap` :`StructRef` _output :`path` _path :`flag` _flag :`Pos1` _pos1 :`Pos2` true :`initialLocation` _initiallocation :!label _label_10)
  (setmembers `/Game/3S_BP/struct_forMap` :`StructRef` _output_2 :`path` _path_2 :`flag` _flag_2 :`Pos1` _pos1_2 :`Pos2` true :`initialLocation` _initiallocation_2)
  (setmembers `/Game/3S_BP/struct_forMap` :`StructRef` _output_3 :`path` _path_3 :`flag` _flag_3 :`Pos1` _pos1_3 :`Pos2` true :`initialLocation` _initiallocation_3)
  (setmembers `/Game/3S_BP/struct_forMap` :`StructRef` _output_4 :`path` _path_4 :`flag` _flag_4 :`Pos1` _pos1_4 :`Pos2` true :`initialLocation` _initiallocation_4)
  (if (and (!= (`self.clear ?`) true) (== (+ _flag _flag_2 _flag_3 _flag_4) 0))
    (`KismetSystemLibrary.PrintString` "fail" true true (struct :`R` 1.0 :`A` 1.0))))

(event `self.collision_J.OnComponentEndOverlap`
  (params (OverlappedComponent :type "PrimitiveComponent Object Reference") (OtherActor :type "Actor Object Reference") (OtherComp :type "PrimitiveComponent Object Reference") (OtherBodyIndex :type Integer))
  (goto _label_10))

(event `self.collision_K.OnComponentBeginOverlap`
  (params (OverlappedComponent :type "PrimitiveComponent Object Reference") (OtherActor :type "Actor Object Reference") (OtherComp :type "PrimitiveComponent Object Reference") (OtherBodyIndex :type Integer) (bFromSweep :type Boolean) (SweepResult :type "HitResult Structure (by ref)"))
  (bind _output (`|GetArrayItem` (`self.paths`) 9))
  (bind _output_2 (`|GetArrayItem` (`self.paths`)))
  (bind _output_3 (`|GetArrayItem` (`self.paths`) 2))
  (bind _output_4 (`|GetArrayItem` (`self.paths`) 4))
  (bind (_path _flag _pos1 _pos2 _initiallocation) (break `/Game/3S_BP/struct_forMap` _output))
  (bind (_path_2 _flag_2 _pos1_2 _pos2_2 _initiallocation_2) (break `/Game/3S_BP/struct_forMap` _output_2))
  (bind (_path_3 _flag_3 _pos1_3 _pos2_3 _initiallocation_3) (break `/Game/3S_BP/struct_forMap` _output_3))
  (bind (_path_4 _flag_4 _pos1_4 _pos2_4 _initiallocation_4) (break `/Game/3S_BP/struct_forMap` _output_4))
  (setmembers `/Game/3S_BP/struct_forMap` :`StructRef` _output_2 :`path` _path_2 :`flag` _flag_2 :`Pos1` _pos1_2 :`Pos2` true :`initialLocation` _initiallocation_2 :!label _label_11)
  (setmembers `/Game/3S_BP/struct_forMap` :`StructRef` _output_3 :`path` _path_3 :`flag` _flag_3 :`Pos1` _pos1_3 :`Pos2` true :`initialLocation` _initiallocation_3)
  (setmembers `/Game/3S_BP/struct_forMap` :`StructRef` _output_4 :`path` _path_4 :`flag` _flag_4 :`Pos1` _pos1_4 :`Pos2` true :`initialLocation` _initiallocation_4)
  (setmembers `/Game/3S_BP/struct_forMap` :`StructRef` _output :`path` _path :`flag` _flag :`Pos1` _pos1 :`Pos2` true :`initialLocation` _initiallocation)
  (if (and (!= (`self.clear ?`) true) (== (+ _flag_2 _flag_3 _flag_4 _flag) 0))
    (`KismetSystemLibrary.PrintString` "fail" true true (struct :`R` 1.0 :`A` 1.0))))

(event `self.collision_K.OnComponentEndOverlap`
  (params (OverlappedComponent :type "PrimitiveComponent Object Reference") (OtherActor :type "Actor Object Reference") (OtherComp :type "PrimitiveComponent Object Reference") (OtherBodyIndex :type Integer))
  (goto _label_11))

(event `self.collision_L.OnComponentBeginOverlap`
  (params (OverlappedComponent :type "PrimitiveComponent Object Reference") (OtherActor :type "Actor Object Reference") (OtherComp :type "PrimitiveComponent Object Reference") (OtherBodyIndex :type Integer) (bFromSweep :type Boolean) (SweepResult :type "HitResult Structure (by ref)"))
  (bind _output (`|GetArrayItem` (`self.paths`) 1))
  (bind _output_2 (`|GetArrayItem` (`self.paths`) 11))
  (bind _output_3 (`|GetArrayItem` (`self.paths`) 5))
  (bind (_path _flag _pos1 _pos2 _initiallocation) (break `/Game/3S_BP/struct_forMap` _output_3))
  (bind (_path_2 _flag_2 _pos1_2 _pos2_2 _initiallocation_2) (break `/Game/3S_BP/struct_forMap` _output))
  (bind (_path_3 _flag_3 _pos1_3 _pos2_3 _initiallocation_3) (break `/Game/3S_BP/struct_forMap` _output_2))
  (setmembers `/Game/3S_BP/struct_forMap` :`StructRef` _output :`path` _path_2 :`flag` _flag_2 :`Pos1` _pos1_2 :`Pos2` true :`initialLocation` _initiallocation_2 :!label _label_12)
  (setmembers `/Game/3S_BP/struct_forMap` :`StructRef` _output_3 :`path` _path :`flag` _flag :`Pos1` _pos1 :`Pos2` true :`initialLocation` _initiallocation)
  (setmembers `/Game/3S_BP/struct_forMap` :`StructRef` _output_2 :`path` _path_3 :`flag` _flag_3 :`Pos1` _pos1_3 :`Pos2` true :`initialLocation` _initiallocation_3)
  (if (and (!= (`self.clear ?`) true) (== (+ _flag _flag_3) 0))
    (`KismetSystemLibrary.PrintString` "fail" true true (struct :`R` 1.0 :`A` 1.0))))

(event `self.collision_L.OnComponentEndOverlap`
  (params (OverlappedComponent :type "PrimitiveComponent Object Reference") (OtherActor :type "Actor Object Reference") (OtherComp :type "PrimitiveComponent Object Reference") (OtherBodyIndex :type Integer))
  (goto _label_12))

(fn `UserConstructionScript`)