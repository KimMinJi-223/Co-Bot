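; Maze puzzle actor that slides a cube along world X and Y while something overlaps its four directional trigger volumes.
; Begin and end overlap events on the forward, back, right and left triggers set direction flags.
; Each tick turns the flags into a fixed per-frame step, blocked when that side's probe collision cube overlaps the Maze component, with forward and right taking priority over their opposites.
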(event `self.ReceiveTick`
  (params (DeltaSeconds :type "Float (single-precision)"))
  (if (`self.Is_forward`)
    (if (not (`PrimitiveComponent.IsOverlappingComponent` (`self.collision_cube_forward`) (`self.maze`)))
      (set `self.move_forward` 1.0))
    (elif (`self.Is_back`)
      (if (not (`PrimitiveComponent.IsOverlappingComponent` (`self.collision_cube_back`) (`self.maze`)))
        (set `self.move_forward` -1.0))))
  (if (`self.Is_right`)
    (if (not (`PrimitiveComponent.IsOverlappingComponent` (`self.collision_cube_right`) (`self.maze`)))
      (set `self.move_right` 1.0))
    (elif (`self.Is_left`)
      (if (not (`PrimitiveComponent.IsOverlappingComponent` (`self.collision_cube_left`) (`self.maze`)))
        (set `self.move_right` -1.0))))
  (`SceneComponent.K2_AddWorldOffset` (`self.Cube`) (`KismetMathLibrary.MakeVector` (`self.move_forward`) (`self.move_right`)) false false)
  (set `self.move_right` 0.0)
  (set `self.move_forward` 0.0))

(event `self.collision_forward.OnComponentBeginOverlap`
  (params (OverlappedComponent :type "PrimitiveComponent Object Reference") (OtherActor :type "Actor Object Reference") (OtherComp :type "PrimitiveComponent Object Reference") (OtherBodyIndex :type Integer) (bFromSweep :type Boolean) (SweepResult :type "HitResult Structure (by ref)"))
  (set `self.Is_forward` true))

(event `self.collision_back.OnComponentBeginOverlap`
  (params (OverlappedComponent :type "PrimitiveComponent Object Reference") (OtherActor :type "Actor Object Reference") (OtherComp :type "PrimitiveComponent Object Reference") (OtherBodyIndex :type Integer) (bFromSweep :type Boolean) (SweepResult :type "HitResult Structure (by ref)"))
  (set `self.Is_back` true))

(event `self.collision_forward.OnComponentEndOverlap`
  (params (OverlappedComponent :type "PrimitiveComponent Object Reference") (OtherActor :type "Actor Object Reference") (OtherComp :type "PrimitiveComponent Object Reference") (OtherBodyIndex :type Integer))
  (set `self.Is_forward` false))

(event `self.collision_back.OnComponentEndOverlap`
  (params (OverlappedComponent :type "PrimitiveComponent Object Reference") (OtherActor :type "Actor Object Reference") (OtherComp :type "PrimitiveComponent Object Reference") (OtherBodyIndex :type Integer))
  (set `self.Is_back` false))

(event `self.collision_right.OnComponentBeginOverlap`
  (params (OverlappedComponent :type "PrimitiveComponent Object Reference") (OtherActor :type "Actor Object Reference") (OtherComp :type "PrimitiveComponent Object Reference") (OtherBodyIndex :type Integer) (bFromSweep :type Boolean) (SweepResult :type "HitResult Structure (by ref)"))
  (set `self.Is_right` true))

(event `self.collision_left.OnComponentBeginOverlap`
  (params (OverlappedComponent :type "PrimitiveComponent Object Reference") (OtherActor :type "Actor Object Reference") (OtherComp :type "PrimitiveComponent Object Reference") (OtherBodyIndex :type Integer) (bFromSweep :type Boolean) (SweepResult :type "HitResult Structure (by ref)"))
  (set `self.Is_left` true))

(event `self.collision_right.OnComponentEndOverlap`
  (params (OverlappedComponent :type "PrimitiveComponent Object Reference") (OtherActor :type "Actor Object Reference") (OtherComp :type "PrimitiveComponent Object Reference") (OtherBodyIndex :type Integer))
  (set `self.Is_right` false))

(event `self.collision_left.OnComponentEndOverlap`
  (params (OverlappedComponent :type "PrimitiveComponent Object Reference") (OtherActor :type "Actor Object Reference") (OtherComp :type "PrimitiveComponent Object Reference") (OtherBodyIndex :type Integer))
  (set `self.Is_left` false))

(fn `UserConstructionScript`)