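; BP_gearkey_2S is a gear key actor with Forward and Back trigger components that track overlaps.
; Overlap begin and end on each component set or clear the IsForward and IsBack flags, without filtering the overlapping actor.
; Tick branches on both flags, but every branch is empty and the AddWorldOffset node is disconnected, so the Blueprint performs no movement.
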(event `self.ReceiveTick`
  (params (DeltaSeconds :type "Float (single-precision)"))
  (bind _is_back (`self.Is_back`))
  (if (`self.Is_forward`)
    (if _is_back
      _)
    (elif _is_back
      _)))

(event `self.forward.OnComponentBeginOverlap`
  (params (OverlappedComponent :type "PrimitiveComponent Object Reference") (OtherActor :type "Actor Object Reference") (OtherComp :type "PrimitiveComponent Object Reference") (OtherBodyIndex :type Integer) (bFromSweep :type Boolean) (SweepResult :type "HitResult Structure (by ref)"))
  (set `self.Is_forward` true))

(event `self.forward.OnComponentEndOverlap`
  (params (OverlappedComponent :type "PrimitiveComponent Object Reference") (OtherActor :type "Actor Object Reference") (OtherComp :type "PrimitiveComponent Object Reference") (OtherBodyIndex :type Integer))
  (set `self.Is_forward` false))

(event `self.back.OnComponentBeginOverlap`
  (params (OverlappedComponent :type "PrimitiveComponent Object Reference") (OtherActor :type "Actor Object Reference") (OtherComp :type "PrimitiveComponent Object Reference") (OtherBodyIndex :type Integer) (bFromSweep :type Boolean) (SweepResult :type "HitResult Structure (by ref)"))
  (set `self.Is_back` true))

(event `self.back.OnComponentEndOverlap`
  (params (OverlappedComponent :type "PrimitiveComponent Object Reference") (OtherActor :type "Actor Object Reference") (OtherComp :type "PrimitiveComponent Object Reference") (OtherBodyIndex :type Integer))
  (set `self.Is_back` false))

(fn `UserConstructionScript`)