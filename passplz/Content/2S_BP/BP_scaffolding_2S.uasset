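; Pressure-plate (foothold) Blueprint that opens a door once enough overlaps are registered on it.
; Box begin and end overlaps raise and lower FootNum, with no filter on what overlaps.
; When a new overlap brings FootNum to DooropenNum, MoveComponentTo slides Door to a raised relative position and Box collision is disabled, with no closing logic.
; An older per-frame offset version using IsDoorUp remains as unexecuted nodes.
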(event `self.ReceiveTick`
  (params (DeltaSeconds :type "Float (single-precision)"))
  ;[1 0.9755 0.3231] 삭제 해도 될듯
)

(event `self.Box.OnComponentBeginOverlap`
  (params (OverlappedComponent :type "PrimitiveComponent Object Reference") (OtherActor :type "Actor Object Reference") (OtherComp :type "PrimitiveComponent Object Reference") (OtherBodyIndex :type Integer) (bFromSweep :type Boolean) (SweepResult :type "HitResult Structure (by ref)"))
  ;[0 1 0.4967] Cpp 완료 여기 무한 호출한다...앞에 set부분 없으면 무한 호출... 이거 딱 멈추는데 아니고 누르고 있으면 계속 앞으로 가는걸로 할까? sky생성 팩토리에서는 위치가 아닌 시간으로 움직임을 결정하는 걸로하는게 정신건강에 좋을듯..
  ;;[1 1 1] 발판 위에 뭔가 올라왔을때 판단한다.
  (set `self.foot_num` (+ (`self.foot_num`) 1))
  (if (== (`self.foot_num`) (`self.dooropen_num`))
    (`KismetSystemLibrary.MoveComponentTo` (`self.door`) (0.0 0.0 200.0) (struct) false false 5.0)
    (`PrimitiveComponent.SetCollisionEnabled` (`self.Box`) "NoCollision")))

(event `self.Box.OnComponentEndOverlap`
  (params (OverlappedComponent :type "PrimitiveComponent Object Reference") (OtherActor :type "Actor Object Reference") (OtherComp :type "PrimitiveComponent Object Reference") (OtherBodyIndex :type Integer))
  ;[0 1 0.4967] Cpp 완료 여기 무한 호출한다...앞에 set부분 없으면 무한 호출... 이거 딱 멈추는데 아니고 누르고 있으면 계속 앞으로 가는걸로 할까? sky생성 팩토리에서는 위치가 아닌 시간으로 움직임을 결정하는 걸로하는게 정신건강에 좋을듯..
  ;;[1 1 1] 발판 위에 뭔가 없어질때 판단
  (set `self.foot_num` (- (`self.foot_num`) 1)))

(fn `UserConstructionScript`)