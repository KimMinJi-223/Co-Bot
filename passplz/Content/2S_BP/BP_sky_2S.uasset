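; BP_sky_2S is an actor that moves along X, with a Box1 trigger volume.
; On overlap, Box1 prints a debug string, disables its collision, and eases the root to X = MoveValue with MoveComponentTo in a repeating loop.
; Tick separately offsets the actor by MoveValue while IsMoving, stopping past an X limit.
; No live node sets IsMoving true, and a note marks the overlap logic as converted to C++.
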(event `self.ReceiveTick`
  (params (DeltaSeconds :type "Float (single-precision)"))
  (if (`self.Is_moving`)
    (`self.K2_AddActorWorldOffset` (`KismetMathLibrary.MakeVector` (`self.move_value`)))
    (set `self.current_move` (+ (`self.current_move`) (`self.move_value`)))
    (if (> (.x (`self.K2_GetActorLocation`)) 4000.0)
      (set `self.Is_moving` false)
      (`PrimitiveComponent.SetCollisionEnabled` (`self.Box1`) "NoCollision"))))

(event `self.Box1.OnComponentBeginOverlap`
  (params (OverlappedComponent :type "PrimitiveComponent Object Reference") (OtherActor :type "Actor Object Reference") (OtherComp :type "PrimitiveComponent Object Reference") (OtherBodyIndex :type Integer) (bFromSweep :type Boolean) (SweepResult :type "HitResult Structure (by ref)"))
  (bind (_returnvalue_x _returnvalue_y _returnvalue_z) (`KismetMathLibrary.BreakVector` (`self.K2_GetActorLocation`)))
  ;[1 1 1] Cpp변환 완료
  (`KismetSystemLibrary.PrintString` "Hello")
  ;[1 1 1] 노콜리전을 더 앞에서 해줘야한다.
  (`PrimitiveComponent.SetCollisionEnabled` (`self.Box1`) "NoCollision" :!label _label)
  (`KismetSystemLibrary.MoveComponentTo` (`self.DefaultSceneRoot`) (`KismetMathLibrary.MakeVector` (`self.move_value`) _returnvalue_y _returnvalue_z) (struct) false false 5.0)
  (goto _label))

(event `self.Box1.OnComponentEndOverlap`
  (params (OverlappedComponent :type "PrimitiveComponent Object Reference") (OtherActor :type "Actor Object Reference") (OtherComp :type "PrimitiveComponent Object Reference") (OtherBodyIndex :type Integer)))

(fn `UserConstructionScript`)